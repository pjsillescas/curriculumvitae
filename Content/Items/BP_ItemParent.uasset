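; Base item actor that the player can pick up, inspect and drop.
; Interacting attaches it to the player's grip with physics off, or starts inspection if the player already holds an item.
; Inspection swaps player input and HUD for its own, placing the item before the camera for mouse-drag rotation and wheel zoom.
; Interact exits inspection, zeroing relative transform; Drop detaches it in front of the camera and restores physics.
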(event EventBeginPlay)

(event Collision|EventActorBeginOverlap
  (params (OtherActor :type Actor%20Object%20Reference)))

(event EventTick
  (params (DeltaSeconds :type Float%20%28single-precision%29)))

(event EventLookat
  (params (PlayerCharacter :type First%20Person%20Character%20Object%20Reference))
  (Default|UpdateMessage (Variables|/Game/FirstPersonBP/Blueprints/FirstPersonCharacter.FirstPersonCharacter_C|GetHud PlayerCharacter) (Utilities|Text|FormatText "Press F to pickup {name}" (Variables|Default|GetItemName))))

(event EventInteractwith
  (params (PlayerCharacter :type First%20Person%20Character%20Object%20Reference))
  (Development|PrintString (Utilities|GetObjectName self))
  (bind _output_get (Variables|Default|SetPlayer PlayerCharacter))
  (Variables|/Game/FirstPersonBP/Blueprints/FirstPersonCharacter.FirstPersonCharacter_C|GetCurrentlyHeldItem _output_get
    (:then
      (CallFunction|StartInspect)
      (Development|PrintString "Inspect"))
    (:else
      (CallFunction|PickUpItem)
      (Development|PrintString "Pickup"))))

(event Input|ActionEvents|InputActionInteract
  (params (Key :type Key%20Structure :default "None"))
  (:Pressed
    (CallFunction|StopInspect)))

(event Input|MouseEvents|MouseX
  (params (AxisValue :type Float%20%28single-precision%29))
  (CallFunction|UpdateRotation (Math|Rotator|MakeRotator 0.0 0.0 (* AxisValue -5.0))))

(event Input|MouseEvents|MouseY
  (params (AxisValue :type Float%20%28single-precision%29))
  (CallFunction|UpdateRotation (Math|Rotator|MakeRotator 0.0 (* AxisValue -5.0) 0.0)))

(event Input|MouseEvents|LeftMouseButton
  (params (Key :type Key%20Structure :default "None"))
  (:Pressed
    (Variables|Default|SetbIsRotating true))
  (:Released
    (Variables|Default|SetbIsRotating false)))

(event Input|MouseEvents|MouseWheelUp
  (params (Key :type Key%20Structure :default "None"))
  (:Pressed
    (CallFunction|UpdateZoom 1)))

(event Input|MouseEvents|MouseWheelDown
  (params (Key :type Key%20Structure :default "None"))
  (:Pressed
    (CallFunction|UpdateZoom -1)))

(fn ConstructionScript)

(fn PickUpItem
  (bind _staticmesh (Variables|Default|GetStaticMesh))
  (Physics|SetSimulatePhysics _staticmesh false)
  (Collision|SetCollisionEnabled _staticmesh "NoCollision")
  (Transformation|AttachComponentToComponent (Variables|/Game/FirstPersonBP/Blueprints/FirstPersonCharacter.FirstPersonCharacter_C|GetItemGrip (Variables|Default|GetPlayer)) "None" "SnapToTarget" "SnapToTarget" "KeepRelative" true)
  (Variables|/Game/FirstPersonBP/Blueprints/FirstPersonCharacter.FirstPersonCharacter_C|SetCurrentlyHeldItem (Variables|Default|GetPlayer) self))

(fn StartInspect
  (bind _returnvalue (Game|GetPlayerController 0))
  (CallFunction|CreateWidget)
  (Input|DisableInput (Variables|Default|GetPlayer) _returnvalue)
  (Input|EnableInput _returnvalue)
  (CallFunction|UpdateActorLocation (Variables|Default|GetTraceLength)))

(fn Drop
  (bind _staticmesh (Variables|Default|GetStaticMesh))
  (Transformation|DetachFromActor "KeepWorld" "KeepWorld" "KeepWorld")
  (CallFunction|UpdateActorLocation (Variables|Default|GetTraceLength))
  (Physics|SetSimulatePhysics _staticmesh true)
  (Collision|SetCollisionEnabled _staticmesh "QueryAndPhysics"))

(fn UpdateActorLocation
  (params (TraceLength :type Float%20%28single-precision%29))
  (bind _returnvalue (Game|GetPlayerCameraManager 0))
  (Transformation|SetActorLocation (+ (Camera|GetCameraLocation _returnvalue) (* (Math|Vector|GetForwardVector (Camera|GetCameraRotation _returnvalue)) TraceLength)) false false))

(fn UpdateRotation
  (params (B :type Rotator))
  (if (Variables|Default|GetbIsRotating)
    (Transformation|SetActorRotation (Math|Rotator|CombineRotators (Transformation|GetActorRotation) B))))

(fn UpdateZoom
  (params (DeltaZoom :type Integer))
  (bind _output_get (Variables|Default|SetZoomLevel (Math|Integer|Clamp(Integer) (+ DeltaZoom (Variables|Default|GetZoomLevel)) 1 (Variables|Default|GetMaxZoom))))
  (if (and (> _output_get 1) (< _output_get (Variables|Default|GetMaxZoom)))
    (CallFunction|UpdateActorLocation (* (Variables|Default|GetZoomLevel) (/ (Variables|Default|GetTraceLength) (Math|Conversions|ToFloat(Integer) (Variables|Default|GetMaxZoom)))))))

(fn StopInspect
  (bind _returnvalue (Game|GetPlayerController 0))
  (Input|DisableInput _returnvalue)
  (Input|EnableInput (Variables|Default|GetPlayer) _returnvalue)
  (Transformation|SetActorRelativeLocation "0, 0, 0")
  (Transformation|SetActorRelativeRotation "0, 0, 0")
  (Widget|RemovefromParent (Variables|Default|GetInspectionHud))
  (Widget|SetVisibility (Variables|/Game/FirstPersonBP/Blueprints/FirstPersonCharacter.FirstPersonCharacter_C|GetHud (Variables|Default|GetPlayer)) "Visible"))

(fn CreateWidget
  (Widget|SetVisibility (Variables|/Game/FirstPersonBP/Blueprints/FirstPersonCharacter.FirstPersonCharacter_C|GetHud (Variables|Default|GetPlayer)) "Hidden")
  (bind _returnvalue (UserInterface|CreateWidget "/Game/Items/UI/WBP_InspectionScreen.WBP_InspectionScreen_C" (Game|GetPlayerController 0) (Variables|Default|GetItemDescription)))
  (bind _output_get (Variables|Default|SetInspectionHud _returnvalue))
  (UserInterface|Viewport|AddtoViewport _output_get 0))