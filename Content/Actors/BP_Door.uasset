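; BP_Door is a locked door actor that opens when the player interacts while holding the matching Key item.
; Lookat sends a HUD prompt built by GetText, naming the needed key or the use key, and blank once open.
; Interactwith triggers OpenDoor, consumes the held item and sets IsOpen.
; A timeline moves the mesh on local Z, adding DoorHeight times OpenHeight as a relative offset every update.
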(event Custom|OpenDoor
  (bind _doorheight (Timeline|TLDoorPosition Play)
    (:Update
      (Transformation|AddLocalOffset (Variables|Debug|GetStaticMeshComponent) (Math|Vector|MakeVector 0.0 0.0 (* _doorheight (Variables|Default|GetOpenHeight))) false false))))

(event EventBeginPlay)

(event Collision|EventActorBeginOverlap
  (params (OtherActor :type Actor%20Object%20Reference)))

(event EventTick
  (params (DeltaSeconds :type Float%20%28single-precision%29)))

(event EventLookat
  (params (PlayerCharacter :type First%20Person%20Character%20Object%20Reference))
  (Default|UpdateMessage (Variables|/Game/FirstPersonBP/Blueprints/FirstPersonCharacter.FirstPersonCharacter_C|GetHud PlayerCharacter) (CallFunction|GetText PlayerCharacter)))

(event EventInteractwith
  (params (PlayerCharacter :type First%20Person%20Character%20Object%20Reference))
  (if (and (== (Variables|/Game/FirstPersonBP/Blueprints/FirstPersonCharacter.FirstPersonCharacter_C|GetCurrentlyHeldItem PlayerCharacter) (Variables|Default|GetKey)) (not (Variables|Default|GetbIsOpen)))
    (CallFunction|OpenDoor)
    (Default|DestroyCurrentItem PlayerCharacter)
    (Variables|Default|SetbIsOpen true)))

(fn ConstructionScript)

(fn GetText
  (params (Character :type First%20Person%20Character%20Object%20Reference))
  (bind _currentlyhelditem (Variables|/Game/FirstPersonBP/Blueprints/FirstPersonCharacter.FirstPersonCharacter_C|GetCurrentlyHeldItem Character))
  (bind _key (Variables|Default|GetKey))
  (if (Variables|Default|GetbIsOpen)
    (return "")
    (elif (== _currentlyhelditem _key)
      (return (Utilities|Text|FormatText "Press F to use {name}" (Variables|/Game/Items/BP_ItemParent.BP_ItemParent_C|GetItemName _currentlyhelditem)))
      (else
        (return (Utilities|Text|FormatText "You need a {name}" (Variables|/Game/Items/BP_ItemParent.BP_ItemParent_C|GetItemName _key)))))))